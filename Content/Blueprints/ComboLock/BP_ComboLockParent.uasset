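; Parent Blueprint for a three-dial combination lock puzzle that opens a safe door.
; ActivatePuzzle blends the view to the lock and enables cursor clicks; the 1 key returns view and input to BP_PersonalProjChar.
; A clicked component's name selects which dial to increment, wrapping at ten, updating its text and animating a rotation step by timeline.
; Each increment compares the concatenated digits against Combo, and a match swings the door via a delayed timeline.
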(event `ActivatePuzzle`
  (bind _returnvalue (`GameplayStatics.GetPlayerController` 0))
  (`PlayerController.SetViewTargetWithBlend` (`GameplayStatics.GetPlayerController` 0) self 1.0 "VTBlend_Linear" 0.0 false)
  (`KismetSystemLibrary.Delay` 1.0)
  (`self.EnableInput` _returnvalue)
  (set `PlayerController.bShowMouseCursor` true _returnvalue)
  (set `PlayerController.bEnableClickEvents` true _returnvalue))

(event `IncrementMove`
  (params (ButtonIn :type "StaticMeshComponent Object Reference"))
  (bind (_returnvalue_roll _returnvalue_pitch) (`KismetMathLibrary.BreakRotator` (`SceneComponent.K2_GetComponentRotation` ButtonIn)))
  (bind _currentrotation (`self.CurrentRotation`))
  (set `self.CurrentRotation` _returnvalue_pitch)
  (bind (_direction _newtrack_0) (`Timeline|Timeline` :!via `PlayFromStart`)
    (:`Update`
      (`SceneComponent.K2_SetRelativeRotation` ButtonIn (`KismetMathLibrary.MakeRotator` 0.0 (`KismetMathLibrary.Lerp` _currentrotation (+ _currentrotation 36.0) _newtrack_0)) false false))))

(event `Key|One`
  (params (Key :type "Key Structure"))
  (bind _returnvalue (`GameplayStatics.GetPlayerController` 0))
  (:`Pressed`
    (set `PlayerController.bShowMouseCursor` false _returnvalue)
    (set `PlayerController.bEnableClickEvents` false _returnvalue)
    (`self.DisableInput` _returnvalue)
    (bind _returnvalue_2 (`GameplayStatics.GetActorOfClass` "/Game/ThirdPerson/Blueprints/BP_PersonalProjChar.BP_PersonalProjChar_C"))
    (`PlayerController.SetViewTargetWithBlend` _returnvalue _returnvalue_2 0.0 "VTBlend_Linear" 0.0 false)
    (`self.EnableInput` _returnvalue_2 _returnvalue)))

(event `self.ReceiveActorOnClicked`
  (params (ButtonPressed :type "Key Structure"))
  (bind (_hitresult _returnvalue) (`PlayerController.GetHitResultUnderCursorForObjects` (`GameplayStatics.GetPlayerController` 0) (`|MakeArray` "ObjectTypeQuery2" :!type "EObjectTypeQuery Enum") true))
  (`KismetSystemLibrary.PrintString` "we are clicking")
  (if _returnvalue
    (`self.Increment` (`KismetSystemLibrary.GetObjectName` (`.HitComponent` (`GameplayStatics.BreakHitResult` _hitresult))))))

(event `Action`
  (params (ActionOn :type Boolean))
  (bind (_returnvalue_roll _returnvalue_pitch) (`KismetMathLibrary.BreakRotator` (`SceneComponent.K2_GetComponentRotation` (`self.SafeDoor`))))
  (if ActionOn
    (`KismetSystemLibrary.Delay` 1.0)
    (bind (_direction _newtrack_0) (`Timeline|Timeline_0`)
      (:`Update`
        (`SceneComponent.K2_SetRelativeRotation` (`self.SafeDoor`) (`KismetMathLibrary.MakeRotator` 0.0 0.0 (`KismetMathLibrary.Lerp` _returnvalue_pitch (+ _returnvalue_pitch -90.0) _newtrack_0)) false false)))))

(fn `CheckCombo`
  (returns (ActionOn :type Boolean))
  (return (`KismetStringLibrary.EqualEqual_StrStr` (`self.Combo`) (`KismetStringLibrary.Concat_StrStr` (`KismetStringLibrary.Conv_IntToString` (`self.Button1Value`)) (`KismetStringLibrary.Conv_IntToString` (`self.Button2Value`)) (`KismetStringLibrary.Conv_IntToString` (`self.Button3Value`))))))

(fn `Increment`
  (params (ButtonName :type String))
  (switch `string` ButtonName
    (:`Default`
      (`KismetSystemLibrary.PrintString` "Fuck you Switch" true true (struct :`R` 1.0 :`B` 0.054508 :`A` 1.0)))
    (:`Button1`
      (bind _output_get (set `self.Button1Value` (mod (+ (`self.Button1Value`) 1) 10)))
      (`TextRenderComponent.K2_SetText` (`self.Button1Text`) (`KismetTextLibrary.Conv_IntToText` _output_get))
      (`self.IncrementMove` (`self.Button1`))
      (bind _actionon (`self.CheckCombo` :!label _label))
      (`self.Action` _actionon)
      (return))
    (:`Button2`
      (bind _output_get_2 (set `self.Button2Value` (mod (+ (`self.Button2Value`) 1) 10)))
      (`TextRenderComponent.K2_SetText` (`self.Button2Text`) (`KismetTextLibrary.Conv_IntToText` _output_get_2))
      (`self.IncrementMove` (`self.Button2`))
      (goto _label))
    (:`Button3`
      (bind _output_get_3 (set `self.Button3Value` (mod (+ (`self.Button3Value`) 1) 10)))
      (`TextRenderComponent.K2_SetText` (`self.Button3Text`) (`KismetTextLibrary.Conv_IntToText` _output_get_3))
      (`self.IncrementMove` (`self.Button3`))
      (goto _label))))

(fn `UserConstructionScript`)