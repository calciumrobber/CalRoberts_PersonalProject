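; Combo lock puzzle Blueprint that animates its three buttons and opens a referenced door when its action fires.
; IncrementMove lights the passed button, picks its hardcoded base location by object name, and plays one shared timeline that offsets it along Y, then dulls its material on finish.
; When Action receives true, it turns the light green, briefly delays, calls OpenDoor on the door reference and ends the puzzle.
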(event `self.IncrementMove`
  (params (ButtonIn :type "StaticMeshComponent Object Reference"))
  (bind _buttonlocation (`self.ButtonLocation`))
  (bind _output_get (set `self.Button In` ButtonIn))
  (`PrimitiveComponent.SetMaterial` _output_get 0 "/Game/Materials/MI_EmissiveOffWhite.MI_EmissiveOffWhite")
  (switch `string` (`KismetSystemLibrary.GetObjectName` ButtonIn)
    (:`Button1`
      (set `self.ButtonLocation` (25.0 100.0 40.0))
      (bind (_direction _newtrack_0) (`Timeline|Timeline_1` :!via `PlayFromStart` :!label _label)
        (:`Update`
          (`SceneComponent.K2_SetRelativeLocation` (`self.Button In`) (`KismetMathLibrary.VLerp` _buttonlocation (+ _buttonlocation (0.0 -8.0 0.0)) _newtrack_0) false false))
        (:`Finished`
          (`PrimitiveComponent.SetMaterial` (`self.Button In`) 0 "/Game/Materials/MI_EmissiveDull.MI_EmissiveDull"))))
    (:`Button2`
      (set `self.ButtonLocation` (50.0 100.0 40.0))
      (goto _label :!via `PlayFromStart`))
    (:`Button3`
      (set `self.ButtonLocation` (75.0 100.0 40.0))
      (goto _label :!via `PlayFromStart`))))

(event `self.Action`
  (params (ActionOn :type Boolean))
  (if ActionOn
    (`PrimitiveComponent.SetMaterial` (`self.Light`) 0 "/Game/Materials/MI_EmissiveGreen.MI_EmissiveGreen")
    (`KismetSystemLibrary.Delay` 0.2)
    (`/Game/Blueprints/ComboLock/BP_ComboDoor.OpenDoor` (`self.DoorRef`))
    (`self.EndPuzzle`)))

(fn `UserConstructionScript`
  (`parent.UserConstructionScript`))