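; Sliding combination lock puzzle Blueprint that animates the dials and the latch that opens on completion.
; IncrementMove uses a timeline to roll the given dial component back 36 degrees, one tenth of a turn, from its current world roll.
; When Action receives true, a short delay precedes a second timeline that slides the latch along local X, then calls EndPuzzle when finished.
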(event `self.Action`
  (params (ActionOn :type Boolean))
  (if ActionOn
    (`KismetSystemLibrary.Delay` 0.5)
    (set `self.LatchLocation` (`SceneComponent.K2_GetComponentLocation` (`self.Latch`)))
    (bind (_direction _newtrack_0) (`Timeline|LatchMove` :!via `PlayFromStart`)
      (:`Update`
        (`SceneComponent.K2_SetRelativeLocation` (`self.Latch`) (`KismetMathLibrary.VLerp` (5.0 0.0 12.0) (32.0 0.0 12.0) _newtrack_0) false false))
      (:`Finished`
        (`self.EndPuzzle`)))))

(event `self.IncrementMove`
  (params (ButtonIn :type "StaticMeshComponent Object Reference"))
  (bind _returnvalue_roll (`KismetMathLibrary.BreakRotator` (`SceneComponent.K2_GetComponentRotation` ButtonIn)))
  (bind _dialrotation (`self.DialRotation`))
  (set `self.DialRotation` _returnvalue_roll)
  (bind (_direction _newtrack_0) (`Timeline|DialMove` :!via `PlayFromStart`)
    (:`Update`
      (`SceneComponent.K2_SetRelativeRotation` ButtonIn (`KismetMathLibrary.MakeRotator` (`KismetMathLibrary.Lerp` _dialrotation (+ _dialrotation -36.0) _newtrack_0)) false false))))

(fn `UserConstructionScript`
  (`parent.UserConstructionScript`))