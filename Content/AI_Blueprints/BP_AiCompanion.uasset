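; AI companion that follows the player's third-person character, which it caches on BeginPlay.
; While its follow flag is set, the FollowPlayer event re-runs on a short delay, using AIMoveTo toward the player beyond a distance threshold.
; Within that range it halts by moving to itself.
; StopMovement reuses that self-targeted move and also feeds back into the follow loop, while BeginPlay does not start the loop.
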(event `self.ReceiveBeginPlay`
  (bind _asbp_third_person_character (cast `/Game/ThirdPerson/Blueprints/BP_ThirdPersonCharacter` (`GameplayStatics.GetPlayerCharacter` 0)))
  (set `self.CharRef` _asbp_third_person_character))

(event `FollowPlayer`
  (if (`self.FollowPlayer?`)
    (if (>= (`self.GetDistanceTo` (`self.CharRef`)) 400.0)
      (`|AIMoveTo` self (0.0 0.0 0.0) (`self.CharRef`)
        (:`then`
          _))
      (else
        (`|AIMoveTo` self (0.0 0.0 0.0) self :!label _label
          (:`then`
            _))))
    (`KismetSystemLibrary.Delay` 0.2)
    (`self.FollowPlayer`)))

(event `StopMovement`
  (goto _label))

(fn `UserConstructionScript`)